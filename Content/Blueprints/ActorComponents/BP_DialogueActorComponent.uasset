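; Actor component that opens and closes a dialogue UI, driven by a DialogueDataTable.
; On BeginPlay it caches the local BP_PretransferPlayerController.
; ShowDialogue creates WBP_Dialogue with the table, adds it to the viewport, blocks look input, shows the cursor and focuses the widget in Game and UI mode.
; HideDialogue removes the widget and restores look input, hidden cursor and game-only input.
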(event Custom|ShowDialogue
  (bind _playercontrollerref (Variables|Default|GetPlayerControllerRef))
  (bind _returnvalue (UserInterface|CreateWidget "/Game/UMG/DialogueWidgets/WBP_Dialogue.WBP_Dialogue_C" 0 (Variables|Default|GetDialogueDataTable)))
  (UserInterface|Viewport|AddtoViewport _returnvalue 0)
  (Variables|Default|SetDialogueWidget _returnvalue)
  (Input|SetIgnoreLookInput _playercontrollerref true)
  (Variables|/Script/Engine.PlayerController|SetbShowMouseCursor _playercontrollerref true)
  (Input|SetInputModeGameandUI _playercontrollerref (Variables|Default|GetDialogueWidget) "DoNotLock" true false))

(event Custom|HideDialogue
  (bind _playercontrollerref (Variables|Default|GetPlayerControllerRef))
  (Widget|RemovefromParent (Variables|Default|GetDialogueWidget))
  (Variables|Default|SetDialogueWidget 0)
  (Input|ResetIgnoreLookInput _playercontrollerref)
  (Variables|/Script/Engine.PlayerController|SetbShowMouseCursor _playercontrollerref false)
  (Input|SetInputModeGameOnly _playercontrollerref false))

(event EventBeginPlay
  (bind _asbp_pretransfer_player_controller (Utilities|Casting|CastToBP_PretransferPlayerController (Game|GetPlayerController 0)))
  (Variables|Default|SetPlayerControllerRef _asbp_pretransfer_player_controller))