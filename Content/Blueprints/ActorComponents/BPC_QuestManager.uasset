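; Quest manager component that runs a linear list of objectives and shows the current one on the main HUD's objectives widget.
; The current objective is always the first uncompleted entry in Objectives, and SetUp stores the HUD reference and displays it.
; FinishObjective completes it only on a matching ID, hiding the widget and optionally showing the next immediately.
; SetNextObjective reveals the current objective when its ID matches.
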(event EventBeginPlay)

(event EventFinishObjective
  (params (ObjectiveID :type Name :default "None") (SetNextObjectiveImmediately :type Boolean))
  (if (== ObjectiveID (.idname (CallFunction|FindObjective)))
    (CallFunction|CompleteObjective)
    (if SetNextObjectiveImmediately
      (CallFunction|SetObjective))))

(event EventSetNextObjective
  (params (ObjectiveID :type Name :default "None"))
  (if (== ObjectiveID (.idname (CallFunction|FindObjective)))
    (CallFunction|SetObjective)))

(fn SetUp
  (params (MainHUDRef :type WBP%20Main%20HUD%20Object%20Reference))
  (Variables|Default|SetMainHUDRef MainHUDRef)
  (CallFunction|SetObjective))

(fn FindObjective
  (bind _array_element (Utilities|Array|ForEachLoopwithBreak (Variables|Default|GetObjectives) :!label _label)
    (:LoopBody
      (if (not (.ObjectiveCompleted (Utilities|Struct|BreakFObjectiveData _array_element)))
        (LocalVariables|SetLocalObjective _array_element)
        (goto _label Break)))
    (:Completed
      (return (LocalVariables|GetLocalObjective)))))

(fn SetObjective
  (bind _mainhudref (Variables|Default|GetMainHUDRef))
  (bind _wbp_objectives (Variables|/Game/UMG/WBP_MainHUD.WBP_MainHUD_C|GetWBP_Objectives _mainhudref))
  (Default|UpdateObjectiveText _wbp_objectives (.objectivetext (CallFunction|FindObjective)))
  (Widget|SetVisibility _wbp_objectives "SelfHitTestInvisible")
  (return))

(fn CompleteObjective
  (bind _foundobjective (CallFunction|FindObjective))
  (bind _objectives (Variables|Default|GetObjectives))
  (bind (_idname _objectivetext) (Utilities|Struct|BreakFObjectiveData _foundobjective))
  (Utilities|Array|SetArrayElem _objectives (Utilities|Array|FindItem _objectives _foundobjective) (Utilities|Struct|MakeFObjectiveData _idname _objectivetext true))
  (Widget|SetVisibility (Variables|/Game/UMG/WBP_MainHUD.WBP_MainHUD_C|GetWBP_Objectives (Variables|Default|GetMainHUDRef)) "Hidden")
  (return))