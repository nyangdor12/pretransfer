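; BP_GrabActor_Base is the base actor for grabbable items in the Pretransfer game.
; BeginPlay casts and caches references to the Pretransfer player controller and player character.
; PerformAction calls LockInPlayer on the controller with the WBP_ExamineActor widget, then runs GrabItem.
; GrabItem adds a BPC Tool System component to the player character at runtime.
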(event EventBeginPlay
  (bind _asbp_pretransfer_player_controller (Utilities|Casting|CastToBP_PretransferPlayerController (Game|GetPlayerController 0)))
  (Variables|Default|SetPlayerControllerRef _asbp_pretransfer_player_controller)
  (bind _asbp_pretransfer_player_character (Utilities|Casting|CastToBP_PretransferPlayerCharacter (Game|GetPlayerCharacter 0)))
  (Variables|Default|SetPlayerRef _asbp_pretransfer_player_character))

(event EventPerformAction
  (Default|LockinPlayer (Variables|Default|GetPlayerControllerRef) "/Game/UMG/WBP_ExamineActor.WBP_ExamineActor_C")
  (CallFunction|GrabItem))

(fn ConstructionScript)

(fn GrabItem
  (AddComponent|AddBPCToolSystem (Variables|Default|GetPlayerRef) false)
  (return))